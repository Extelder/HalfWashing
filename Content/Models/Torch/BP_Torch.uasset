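; BP_Torch is a torch actor that makes its point light flicker during play.
; On BeginPlay it caches the light's starting intensity and plays the Flickering timeline.
; Each update sets the intensity to that base times the timeline curve and a random dimming factor.
; When the timeline finishes, a zero-length delay restarts it from the start, looping the flicker continuously.
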(event EventBeginPlay
  (Variables|Default|Setintensity (Variables|/Script/Engine.LightComponentBase|GetIntensity (Variables|Default|GetPointLight)))
  (bind _intensitytrack (Timeline|Flickering Play)
    (:Update
      (Rendering|Components|Light|SetIntensity (Variables|Default|GetPointLight) (* (* (Variables|Default|Getintensity) _intensitytrack) (Math|Random|RandomFloatinRange 0.7 1.0))))
    (:Finished
      (Utilities|FlowControl|Delay 0.0)
      (Timeline|Flickering PlayFromStart))))

(event Collision|EventActorBeginOverlap
  (params (OtherActor :type Actor%20Object%20Reference)))

(event EventTick
  (params (DeltaSeconds :type Float%20%28single-precision%29)))

(fn ConstructionScript)