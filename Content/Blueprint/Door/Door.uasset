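; Door Blueprint that checks throwable keys entering its KeyTrigger for a matching DoorNum.
; A match calls OpenDoor, which forwards the key to OpenDoorMulticast to destroy it and print a "Door Open" message.
; A non-matching key plays a 2D click sound instead.
; The door itself does not move or change state in this graph, so opening is only a debug print.
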(event OnComponentBeginOverlap(KeyTrigger)
  (params (OverlappedComponent :type Primitive%20Component%20Object%20Reference) (OtherActor :type Actor%20Object%20Reference) (OtherComp :type Primitive%20Component%20Object%20Reference) (OtherBodyIndex :type Integer) (bFromSweep :type Boolean) (SweepResult :type Hit%20Result%20Structure%20%28by%20ref%29))
  (bind _astakable_and_throwable_key (Utilities|Casting|CastToTakableAndThrowable_Key OtherActor))
  (if (== (Variables|/Game/Blueprint/Throwable/TakableAndThrowable_Key.TakableAndThrowable_Key_C|GetDoorNum _astakable_and_throwable_key) (Variables|Default|GetDoorNum))
    (CallFunction|OpenDoor _astakable_and_throwable_key)
    (else
      (Audio|PlaySound2D "/Engine/VREditor/Sounds/UI/Click_on_Button_Cue.Click_on_Button_Cue" 1.0 1.0 0.0 0 0))))

(event Custom|OpenDoor
  (params (Key :type Takable%20and%20Throwable%20Key%20Object%20Reference))
  (CallFunction|OpenDoorMulticast Key))

(event Custom|OpenDoorMulticast
  (params (Target :type Actor%20Object%20Reference))
  (Utilities|IsValid Target
    (:Is%20Valid
      (Actor|DestroyActor Target))
    (:Is%20Not%20Valid
      _))
  (Development|PrintString "Door Open"))

(fn ConstructionScript)