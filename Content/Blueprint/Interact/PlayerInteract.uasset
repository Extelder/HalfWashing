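; Player character component that lets a player interact with, grab, release and throw objects.
; On Tick, the locally controlled player line-traces from the camera to cache the IInteractable in view.
; Interact input toggles Grabbing, passing the PhysicsHandle to that interactable or releasing it through server events.
; Throw input releases the handle and applies a camera-forward impulse to a TakableAndThrowable, using the currently traced target.
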(event Custom|InteractInteractableServer
  (params (Target :type I%20Interactable%20Interface) (PhysicsHandle :type Physics%20Handle%20Component%20Object%20Reference))
  (Default|InteractInteractable Target PhysicsHandle self))

(event Custom|ReleaseOnServer
  (params (Target :type Physics%20Handle%20Component%20Object%20Reference))
  (Physics|Components|PhysicsHandle|ReleaseComponent Target)
  (Variables|Default|SetGrabbing false))

(event Custom|ThrowOnServer
  (params (Target :type Takable%20and%20Throwable%20Object%20Reference))
  (Physics|Components|PhysicsHandle|ReleaseComponent (Variables|/Game/Blueprint/Player/PlayerMain/PlayerCharacter.PlayerCharacter_C|GetPhysicsHandle (Variables|Default|GetPlayerCharacter)))
  (Variables|Default|SetGrabbing false)
  (Physics|AddImpulse (Variables|/Game/Blueprint/Throwable/TakableAndThrowable.TakableAndThrowable_C|GetStaticMesh Target) (* (Math|Vector|GetForwardVector (Variables|/Game/Blueprint/Player/PlayerMain/PlayerCharacter.PlayerCharacter_C|GetCamera (Variables|Default|GetPlayerCharacter))) (Variables|Default|GetThrowForce)) "None" true))

(event EventTick
  (params (DeltaSeconds :type Float%20%28single-precision%29))
  (bind _playercharacter (Variables|Default|GetPlayerCharacter))
  (bind _camera (Variables|/Game/Blueprint/Player/PlayerMain/PlayerCharacter.PlayerCharacter_C|GetCamera _playercharacter))
  (bind _returnvalue (Transformation|GetWorldLocation _camera))
  (bind _asplayer_character (Utilities|Casting|CastToPlayerCharacter (Components|GetOwner)))
  (if (Pawn|IsLocallyControlled _asplayer_character)
    (bind (_outhit _returnvalue_2) (Collision|LineTraceByChannel _returnvalue (+ _returnvalue (* (Math|Vector|GetForwardVector (Pawn|GetControlRotation _playercharacter :!class /Script/Engine.Pawn)) (Variables|Default|GetLengthLineTrace))) "TraceTypeQuery2" false 0 "None" true "(R=1.000000,G=0.000000,B=0.000000,A=1.000000)" "(R=0.000000,G=1.000000,B=0.000000,A=1.000000)" 1.0))
    (if _returnvalue_2
      (bind _asiinteractable (Utilities|Casting|CastToIInteractable (.HitActor (Collision|BreakHitResult _outhit)))
        (:then
          (Variables|Default|SetAs%20IInteractable _asiinteractable))
        (:CastFailed
          (Variables|Default|SetAs%20IInteractable 0 :!label _label)))
      (else
        (goto _label)))))

(event EventBeginPlay
  (bind _asplayer_character (Utilities|Casting|CastToPlayerCharacter (Components|GetOwner)))
  (Variables|Default|SetPlayerCharacter _asplayer_character))

(event Input|ActionEvents|InputActionThrow
  (params (Key :type Key%20Structure :default "None"))
  (:Pressed
    (if (Variables|Default|GetGrabbing)
      (Variables|Default|SetGrabbing false)
      (bind _astakable_and_throwable (Utilities|Casting|CastToTakableAndThrowable (Variables|Default|GetAs%20IInteractable)))
      (CallFunction|ThrowonServer _astakable_and_throwable))))

(event Input|ActionEvents|InputActionInteract2
  (params (Key :type Key%20Structure :default "None"))
  (bind _as_iinteractable (Variables|Default|GetAs%20IInteractable))
  (bind _playercharacter (Variables|Default|GetPlayerCharacter))
  (bind _physicshandle (Variables|/Game/Blueprint/Player/PlayerMain/PlayerCharacter.PlayerCharacter_C|GetPhysicsHandle _playercharacter))
  (:Pressed
    (if (Variables|Default|GetGrabbing)
      (CallFunction|ReleaseonServer _physicshandle)
      (Variables|Default|SetGrabbing false)
      (else
        (Variables|Default|SetGrabbing true)
        (Utilities|IsValid (Utilities|ToObject(Interface) _as_iinteractable)
          (:Is%20Valid
            (CallFunction|InteractInteractableServer _as_iinteractable _physicshandle)))))))