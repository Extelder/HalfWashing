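; Base enemy with a dog animation Blueprint that detects players, attacks, takes damage and dies through AI Blackboard keys.
; BeginPlay seeds walk radius and start point, PawnSensing records the seen player, and zero health sets Death.
; SetState forwards to SetStateMulticast to update the animation state.
; CheckPlayerHealth damages players overlapping its box, and WidgetVis toggles a widget for the local player in one specific state.
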(event OnSeePawn(PawnSensing)
  (params (Pawn :type Pawn%20Object%20Reference))
  (bind _self self)
  (bind _returnvalue (AI|GetAIController _self))
  (bind _returnvalue_2 (AI|GetBlackboard _returnvalue))
  (bind _asplayer_character (Utilities|Casting|CastToPlayerCharacter Pawn))
  (AI|Components|Blackboard|SetValueasObject _returnvalue_2 (Utilities|Name|MakeLiteralName "Player") _asplayer_character)
  (AI|Components|Blackboard|SetValueasBool _returnvalue_2 (Utilities|Name|MakeLiteralName "PlayerDetected") true))

(event Custom|WidgetVis
  (params (On? :type Boolean) (Player :type Player%20Character%20Object%20Reference))
  (bind _returnvalue (not On?))
  (bind _widget (Variables|Default|GetWidget))
  ;[1 1 1] WidgetOn
  (if (Utilities|Enum|Equal(Enum) (Variables|/Game/Models/Enemy/Dog/DogAnimBP.DogAnimBP_C|GetCurrentState (Variables|Default|GetAs%20Dog%20Anim%20BP)) "NewEnumerator3")
    (if (Variables|Default|GetWidgetCanActivate?)
      (if (Pawn|IsLocallyControlled Player)
        (if On?
          (Development|SetHiddeninGame _widget _returnvalue false)
          (else
            (Development|SetHiddeninGame _widget _returnvalue false)))))))

(event Custom|CheckPlayerHealth
  (for _array_element (Collision|GetOverlappingActors (Variables|Default|GetBox) "/Game/Blueprint/Player/PlayerMain/PlayerCharacter.PlayerCharacter_C" :!class /Script/Engine.PrimitiveComponent)
    (Utilities|IsValid (Actor|GetComponentbyClass _array_element "/Game/Blueprint/Player/Health/Health.Health_C")
      (:Is%20Valid
        (Default|TakeDamage (Actor|GetComponentbyClass _array_element "/Game/Blueprint/Player/Health/Health.Health_C") 23.0)))))

(event Custom|SetStateMulticast
  (params (CurrentState :type EnemyState%20Enum :default "NewEnumerator0"))
  (Variables|/Game/Models/Enemy/Dog/DogAnimBP.DogAnimBP_C|SetCurrentState (Variables|Default|GetAs%20Dog%20Anim%20BP) CurrentState))

(event Custom|SetState
  (params (State :type EnemyState%20Enum :default "NewEnumerator0"))
  (CallFunction|SetStateMulticast State))

(event EventTakeDamage
  (params (Damage :type Float%20%28double-precision%29))
  (if (<= (- (Variables|Default|GetHealth) Damage) 0.0)
    (Variables|Default|SetHealth 0.0)
    (AI|Components|Blackboard|SetValueasBool (AI|GetBlackboard (AI|GetAIController self)) (Utilities|Name|MakeLiteralName "Death") true)
    (else
      (Variables|Default|SetHealth (- (Variables|Default|GetHealth) Damage))
      (Development|PrintString "aaaaaaaaaaaaaaaaaaaaaa"))))

(event EventBeginPlay
  (bind _self self)
  (bind _returnvalue (AI|GetAIController _self))
  (bind _returnvalue_2 (AI|GetBlackboard _returnvalue))
  (bind _asdog_anim_bp (Utilities|Casting|CastToDogAnimBP (Components|SkeletalMesh|GetAnimInstance (Variables|Character|GetMesh))))
  (Variables|Default|SetAs%20Dog%20Anim%20BP _asdog_anim_bp)
  (AI|Components|Blackboard|SetValueasFloat _returnvalue_2 (Utilities|Name|MakeLiteralName "WalkRadius") (Variables|Default|GetWalkRadius))
  (AI|Components|Blackboard|SetValueasVector _returnvalue_2 (Utilities|Name|MakeLiteralName "StartPoint") (Transformation|GetActorLocation)))

(fn ConstructionScript)