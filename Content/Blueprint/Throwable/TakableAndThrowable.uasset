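; TakableAndThrowable is a physics prop that can be grabbed and, if flagged breakable, destroyed by damage.
; Interacting stores the passed PhysicsHandle, enables simulation on the static mesh and grabs it.
; Break subtracts damage only when its type matches the prop's, spawning wood or asphalt particles by type and destroying the actor at zero health.
; SetCollision toggles a custom trace channel between overlap and block; MovementOnMulticast is empty.
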(event Custom|MovementOnMulticast)

(event EventSetCollision
  (params (Overlap? :type Boolean))
  (bind _staticmesh (Variables|Default|GetStaticMesh))
  (if Overlap?
    (Collision|SetCollisionResponsetoChannel _staticmesh "ECC_GameTraceChannel1" "ECR_Overlap")
    (else
      (Collision|SetCollisionResponsetoChannel _staticmesh "ECC_GameTraceChannel1" "ECR_Block"))))

(event EventBreak
  (params (TypeDamage :type Breakable%20Enum :default "NewEnumerator0") (Damage :type Float%20%28double-precision%29))
  (bind _returnvalue (Transformation|GetActorLocation))
  (if (Utilities|Enum|Equal(Enum) TypeDamage (Variables|Default|GetType))
    (if (Variables|Default|GetBreakeble?)
      (if (<= (- (Variables|Default|GetBreakableHP) Damage) 0.0)
        (if (Utilities|Enum|Equal(Enum) (Variables|Default|GetType) "NewEnumerator0")
          (Effects|SpawnEmitteratLocation "/Game/Realistic_Starter_VFX_Pack_Vol2/Particles/Hit/P_Wood.P_Wood" _returnvalue "0, 0, 0" "4.000000,4.000000,4.000000")
          (Actor|DestroyActor)
          (else
            (Effects|SpawnEmitteratLocation "/Game/Realistic_Starter_VFX_Pack_Vol2/Particles/Hit/P_Asphalt.P_Asphalt" _returnvalue "0, 0, 0" "4.000000,4.000000,4.000000")
            (Actor|DestroyActor)))
        (else
          (Variables|Default|SetBreakableHP (- (Variables|Default|GetBreakableHP) Damage)))))))

(event EventInteractInteractable
  (params (PhysicsHandle :type Physics%20Handle%20Component%20Object%20Reference) (PlayerInteract :type Player%20Interact%20Object%20Reference))
  (bind _staticmesh (Variables|Default|GetStaticMesh))
  (bind _output_get (Variables|Default|SetPhysicsHandle PhysicsHandle))
  (Physics|SetSimulatePhysics (Variables|Default|GetStaticMesh) true)
  (Physics|Components|PhysicsHandle|GrabComponentatLocationwithRotation _output_get _staticmesh "None" (Transformation|GetWorldLocation _staticmesh) "0, 0, 0"))

(fn ConstructionScript)