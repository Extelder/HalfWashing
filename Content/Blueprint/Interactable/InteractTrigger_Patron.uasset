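; Interactable revolver ammo pickup that holds a count of cartridges (Patron) and loads them into a six-round cylinder, tracked as the player's RevolverHP.
; On press, a pickup that fits entirely is added, triggers the player's reload and destroys itself.
; Otherwise, unless the cylinder is empty, it fills the cylinder, keeps the remainder and updates its model by toggling cartridge mesh visibility for that count.
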(event EventInteractTrigger
  (params (Pressed? :type Boolean) (Player :type Player%20Character%20Object%20Reference))
  (if Pressed?
    (if (>= (- 6 (Variables|/Game/Blueprint/Player/PlayerMain/PlayerCharacter.PlayerCharacter_C|GetRevolverHP Player)) (Variables|Default|GetPatron))
      (Variables|/Game/Blueprint/Player/PlayerMain/PlayerCharacter.PlayerCharacter_C|SetRevolverHP Player (+ (Variables|/Game/Blueprint/Player/PlayerMain/PlayerCharacter.PlayerCharacter_C|GetRevolverHP Player) (Variables|Default|GetPatron)))
      (Default|PatronLost Player)
      (Default|Reload Player)
      (Actor|DestroyActor)
      (elif (not (== (- 6 (Variables|/Game/Blueprint/Player/PlayerMain/PlayerCharacter.PlayerCharacter_C|GetRevolverHP Player)) 6))
        (Variables|Default|SetPatron (- (Variables|Default|GetPatron) (- 6 (Variables|/Game/Blueprint/Player/PlayerMain/PlayerCharacter.PlayerCharacter_C|GetRevolverHP Player))))
        (Variables|/Game/Blueprint/Player/PlayerMain/PlayerCharacter.PlayerCharacter_C|SetRevolverHP Player 6)
        (Default|PatronLost Player)
        (CallFunction|UpdateModel)))))

(fn ConstructionScript
  (|CallParentFunction))

(fn UpdateModel
  (switch int (Variables|Default|GetPatron)
    (:1
      (Rendering|SetVisibility (Variables|Default|GetPatron1Patron4) false true))
    (:2
      (Rendering|SetVisibility (Variables|Default|GetPatron1Patron3) false true))
    (:3
      (Rendering|SetVisibility (Variables|Default|GetPatron1Patron2) false true))
    (:4
      (Rendering|SetVisibility (Variables|Default|GetPatron1Patron1) false true))
    (:5
      (Rendering|SetVisibility (Variables|Default|GetPatron1Patron) false false))
    (:6
      (Rendering|SetVisibility (Variables|Default|GetStaticMesh) true true))))