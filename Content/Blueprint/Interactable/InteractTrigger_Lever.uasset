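; Lever interact trigger that fires the IEvniromentInteractable Interact call on a linked ActorToInteract.
; Pressing plays the LeverActivate timeline to rotate the lever mesh, and releasing reverses it after a brief delay.
; Rotation checks set an Activate flag that blocks further input.
; Activation routes through ActivateMulticast, which hides the prompt widget and triggers the target.
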(event Custom|ActivateMulticast
  (params (Player :type Player%20Character%20Object%20Reference))
  (Variables|Default|SetWidgetCanActivate? false)
  (Development|SetHiddeninGame (Variables|Default|GetWidget) true false)
  (bind _asilever (Utilities|Casting|CastToIEvniromentInteractable (Variables|Default|GetActorToInteract)))
  (Default|Interact _asilever))

(event Custom|Activate
  (params (Player :type Player%20Character%20Object%20Reference))
  (CallFunction|ActivateMulticast Player))

(event EventInteractTrigger
  (params (Pressed? :type Boolean) (Player :type Player%20Character%20Object%20Reference))
  (bind _lever_lever_v2_box_001 (Variables|Default|GetLever_Lever_v2_Box_001))
  (bind _lever_lever_v2_box_001_2 (Variables|Default|GetLever_Lever_v2_Box_001))
  (bind _relativerotation (Variables|/Script/Engine.SceneComponent|GetRelativeRotation _lever_lever_v2_box_001))
  (bind _relativerotation_2 (Variables|/Script/Engine.SceneComponent|GetRelativeRotation _lever_lever_v2_box_001_2))
  (if (not (Variables|Default|GetActivate?))
    (if Pressed?
      (if (and (<= (.pitch _relativerotation) -5.0) (<= (.yaw _relativerotation) -1.8e+02))
        (Utilities|FlowControl|Sequence
          (:then_0
            (Variables|Default|SetActivate? true)
            (CallFunction|Activate Player))
          (:then_1
            (bind _newtrack_0 (Timeline|LeverActivate Play)
              (:Update
                (Transformation|SetRelativeRotation (Variables|Default|GetLever_Lever_v2_Box_001) (Math|Rotator|MakeRotator 0.0 (Math|Float|Lerp 0.0 -1.8e+02 _newtrack_0) 0.0) false false))
              (:Finished
                (if (or (== (.yaw _relativerotation_2) -1.8e+02) (== (.yaw _relativerotation_2) 1.8e+02))
                  (Variables|Default|SetActivate? true)
                  (CallFunction|Activate Player))))))
        (else
          (Timeline|LeverActivate Play)))
      (else
        (Utilities|FlowControl|Delay 0.03)
        (Timeline|LeverActivate Reverse)))))

(fn ConstructionScript
  (|CallParentFunction))