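; BP_Note_1 is an interactable note that displays the Note_1 widget on screen while the interact input is pressed.
; Its InteractTrigger event acts only for a locally controlled player, creating the widget for player controller 0 on press and removing it on release.
; Move and look input are ignored while the note is shown and re-enabled when it closes.
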(event EventInteractTrigger
  (params (Pressed? :type Boolean) (Player :type Player%20Character%20Object%20Reference))
  (bind _returnvalue (Game|GetPlayerController 0))
  (if (Pawn|IsLocallyControlled Player)
    (if Pressed?
      (bind _returnvalue_2 (UserInterface|CreateWidget "/Game/Widgets/Notes/Note_1.Note_1_C" _returnvalue))
      (UserInterface|Viewport|AddtoViewport _returnvalue_2 0)
      (Input|SetIgnoreMoveInput _returnvalue true)
      (Input|SetIgnoreLookInput _returnvalue true)
      (else
        (Widget|RemovefromParent _returnvalue_2)
        (Input|SetIgnoreMoveInput _returnvalue false)
        (Input|SetIgnoreLookInput _returnvalue false)))))

(fn ConstructionScript)