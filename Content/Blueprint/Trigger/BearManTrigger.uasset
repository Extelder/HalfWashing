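; BearManTrigger is a one-shot scare trigger that plays a lightning-style flash sequence and then makes a skeletal figure vanish.
; The first time the PlayerCharacter overlaps the Box, a DoN gate plays the MolniaCue sound in 2D.
; A hardcoded chain of short, uneven Delays then flickers the StaticMesh's visibility, and the last step hides both it and the SkeletalMesh.
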(event OnComponentBeginOverlap(Box)
  (params (OverlappedComponent :type Primitive%20Component%20Object%20Reference) (OtherActor :type Actor%20Object%20Reference) (OtherComp :type Primitive%20Component%20Object%20Reference) (OtherBodyIndex :type Integer) (bFromSweep :type Boolean) (SweepResult :type Hit%20Result%20Structure%20%28by%20ref%29))
  (bind _staticmesh (Variables|Default|GetStaticMesh))
  (Utilities|Casting|CastToPlayerCharacter OtherActor)
  (Utilities|FlowControl|DoN 1
    (:Exit
      (Audio|PlaySound2D "/Game/Blueprint/My_Friends/Characters/God/MolniaCue.MolniaCue" 1.0 1.0 0.0 0 0)
      (Utilities|FlowControl|Delay 0.4)
      (Rendering|SetVisibility _staticmesh true false)
      (Utilities|FlowControl|Delay 0.1)
      (Rendering|SetVisibility _staticmesh false false)
      (Utilities|FlowControl|Delay 0.1)
      (Rendering|SetVisibility _staticmesh true false)
      (Utilities|FlowControl|Delay 0.15)
      (Rendering|SetVisibility _staticmesh false false)
      (Utilities|FlowControl|Delay 0.05)
      (Rendering|SetVisibility _staticmesh true false)
      (Utilities|FlowControl|Delay 0.5)
      (Rendering|SetVisibility _staticmesh false false)
      (Rendering|SetVisibility (Variables|Default|GetSkeletalMesh) false false))))

(fn ConstructionScript)