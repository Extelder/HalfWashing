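; Friendly NPC character that walks a route of MovePoints in order from BeginPlay, performing an animation at each stop.
; A recursive exec loop moves it with AIMoveTo, plays that point's montage for its TimeOnPoint, stops it, then advances.
; The route ends at the first invalid point without wrapping, and a failed move halts it.
; Tick sets the Mooving flag from velocity.
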(event Custom|StartMoving
  (Variables|Default|SetCurrentIndex -1)
  (bind _result (Math|Integer|IncrementInt (Variables|Default|GetCurrentIndex) :!label _label)
    (:%20%20
      (Utilities|IsValid (Utilities|Array|Get(acopy) (Variables|Default|GetMovePoints) _result)
        (:Is%20Valid
          (AI|AIMoveTo self "0, 0, 0" (Utilities|Array|Get(acopy) (Variables|Default|GetMovePoints) _result) 1e+02 false
            (:OnSuccess
              (Animation|PlayAnimMontage (Variables|/Game/Blueprint/My_Friends/NPCMovePoint.NPCMovePoint_C|GetAnimOn (Utilities|Array|Get(acopy) (Variables|Default|GetMovePoints) _result)) 1.0 "None")
              (Utilities|FlowControl|Delay (Variables|/Game/Blueprint/My_Friends/NPCMovePoint.NPCMovePoint_C|GetTimeOnPoint (Utilities|Array|Get(acopy) (Variables|Default|GetMovePoints) _result)))
              (Animation|StopAnimMontage (Variables|/Game/Blueprint/My_Friends/NPCMovePoint.NPCMovePoint_C|GetAnimOn (Utilities|Array|Get(acopy) (Variables|Default|GetMovePoints) _result)))
              (goto _label))))))))

(event EventBeginPlay
  (CallFunction|StartMoving))

(event EventTick
  (params (DeltaSeconds :type Float%20%28single-precision%29))
  (Variables|Default|SetMooving (>= (Math|Vector|VectorLength (Transformation|GetVelocity)) 1.0)))

(fn ConstructionScript)